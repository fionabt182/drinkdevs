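; Base enemy that switches to flying, rises 200 units from its spawn point on BeginPlay, and shoots at the player.
; AI Perception updates start a looping look-at timer and, if the player is in range, a looping shooting timer.
; Each shot stops the look-at timer, traces from the stored spawn location to the player, and spawns a BP_Projectile aimed along that trace.
; Range is only checked on successful sensing; losing sight clears only the look-at timer.
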(event `self.ReceiveBeginPlay`
  (bind _asbp_third_person_character (cast `/Game/ThirdPerson/Blueprints/BP_ThirdPersonCharacter` (`GameplayStatics.GetPlayerCharacter` 0)))
  (set `self.As BP Third Person Character` _asbp_third_person_character)
  (`CharacterMovementComponent.SetMovementMode` (`self.CharacterMovement`) "MOVE_Flying" 0)
  (set `self.Actor location` (`self.K2_GetActorLocation`))
  (`KismetSystemLibrary.K2_SetTimerDelegate` (delegate `Floating`) 0.1))

(event `Floating`
  (bind (_actor_location_x _actor_location_y _actor_location_z) (`KismetMathLibrary.BreakVector` (`self.Actor location`)))
  (bind (_direction _lerp) (`Timeline|Timeline` :!via `PlayFromStart`)
    (:`Update`
      (`self.K2_SetActorLocation` (`KismetMathLibrary.VLerp` (`self.Actor location`) (`KismetMathLibrary.MakeVector` _actor_location_x _actor_location_y (+ _actor_location_z 200.0)) _lerp)))))

(event `self.AIPerception.OnTargetPerceptionUpdated`
  (params (Actor :type "Actor Object Reference") (Stimulus :type "AIStimulus Structure"))
  ;[1 1 1] WatchingTimer
  (if (`.bSuccessfullySensed` (break `AIStimulus` Stimulus))
    (bind _returnvalue (`KismetSystemLibrary.K2_SetTimerDelegate` (delegate `WatchingPlayer`) 0.1 true))
    (set `self.Watching` _returnvalue)
    (if (< (`GameplayStatics.FindNearestActor` (`self.K2_GetActorLocation`) (`|MakeArray` (`self.As BP Third Person Character`) :!type "Actor Object Reference")) 2000.0)
      (bind _returnvalue_2 (`KismetSystemLibrary.K2_SetTimerDelegate` (delegate `Shooting`) 2.0 true))
      (set `self.Shooting timer` _returnvalue_2)
      (else
        (`KismetSystemLibrary.K2_ClearAndInvalidateTimerHandle` (`self.Shooting timer`))))
    (else
      (`KismetSystemLibrary.K2_ClearAndInvalidateTimerHandle` (`self.Watching`)))))

(event `WatchingPlayer`
  ;[1 1 1] WatchingTimer
  (`self.K2_SetActorRotation` (`KismetMathLibrary.FindLookAtRotation` (`self.K2_GetActorLocation`) (`self.K2_GetActorLocation` (`self.As BP Third Person Character`)))))

(event `Shooting`
  (`KismetSystemLibrary.K2_ClearAndInvalidateTimerHandle` (`self.Watching`))
  (bind _outhit (`KismetSystemLibrary.LineTraceSingle` :`Start` (`self.Actor location`) :`End` (`self.K2_GetActorLocation` (`self.As BP Third Person Character`)) :`TraceChannel` "TraceTypeQuery1" :`DrawDebugType` "ForDuration"))
  (bind (_bblockinghit _binitialoverlap _time _distance _location _impactpoint _normal _impactnormal _physmat _hitactor _hitcomponent _hitbonename _bonename _hititem _elementindex _faceindex _tracestart _traceend) (`GameplayStatics.BreakHitResult` _outhit))
  (`|SpawnActorFromClass` "/Game/Zombe/Fi/BP_Projectile.BP_Projectile_C" (`KismetMathLibrary.MakeTransform` _tracestart (`KismetMathLibrary.FindLookAtRotation` _tracestart _traceend)) "Undefined" "MultiplyWithRoot" null (`self.As BP Third Person Character`) null))

(fn `UserConstructionScript`)