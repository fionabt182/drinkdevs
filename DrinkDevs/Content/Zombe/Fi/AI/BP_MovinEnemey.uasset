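; Flying enemy that hovers with animated wings and attacks the player character with projectiles.
; BeginPlay sets flying movement and starts timeline-driven bobbing and wing rotation.
; AI perception starts a look-at timer and, if the player is within range at that update, a looping shot timer that stops the tracking and spawns BP_Projectile toward them.
; Damage stops the hover, runs a death timeline, then rotates the mesh and swaps its material.
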(event `WingsMove`
  (bind (_returnvalue_roll _returnvalue_pitch _returnvalue_yaw) (`KismetMathLibrary.BreakRotator` (`SceneComponent.K2_GetComponentRotation` (`self.Mesh`))))
  (bind (_returnvalue_roll_2 _returnvalue_pitch_2 _returnvalue_yaw_2) (`KismetMathLibrary.BreakRotator` (`SceneComponent.K2_GetComponentRotation` (`self.Mesh`))))
  ;[1 1 1] Wing Movement
  (bind (_direction _wingmovement) (`Timeline|Left_WingMovement` :`NewTime` 0.5)
    (:`Update`
      (`SceneComponent.K2_SetWorldRotation` (`self.LeftWing`) (`KismetMathLibrary.MakeRotator` _returnvalue_roll _returnvalue_pitch (+ _returnvalue_yaw (.z _wingmovement))) false false)
      (bind (_direction_2 _wingmovement_2) (`Timeline|Right_WingMovement` :`NewTime` 0.5)
        (:`Update`
          (`SceneComponent.K2_SetWorldRotation` (`self.RightWing`) (`KismetMathLibrary.MakeRotator` _returnvalue_roll_2 _returnvalue_pitch_2 (+ _returnvalue_yaw_2 (.z _wingmovement_2))) false false))))))

(event `self.ReceiveBeginPlay`
  (`|ExecutionSequence`
    (:`then_0`
      ;[1 1 1] references
      (bind _asbp_third_person_character (cast `/Game/ThirdPerson/Blueprints/BP_ThirdPersonCharacter` (`GameplayStatics.GetPlayerCharacter` 0)))
      (set `self.As BP Third Person Character` _asbp_third_person_character)
      (`CharacterMovementComponent.SetMovementMode` (`self.CharacterMovement`) "MOVE_Flying" 0)
      (set `self.Actor location` (`self.K2_GetActorLocation`))
      ;[1 1 1] floating
      (`KismetSystemLibrary.K2_SetTimerDelegate` (delegate `Floating`) 0.1))
    (:`then_1`
      (`self.WingsMove`))))

(event `Floating`
  (bind (_actor_location_x _actor_location_y _actor_location_z) (`KismetMathLibrary.BreakVector` (`self.Actor location`)))
  ;[1 1 1] floating
  (bind (_direction _lerp) (`Timeline|Timeline` :!via `PlayFromStart` :!label _label)
    (:`Update`
      (`self.K2_SetActorLocation` (`KismetMathLibrary.VLerp` (`self.Actor location`) (`KismetMathLibrary.MakeVector` _actor_location_x _actor_location_y (+ _actor_location_z 200.0)) _lerp)))))

(event `self.AIPerception.OnTargetPerceptionUpdated`
  (params (Actor :type "Actor Object Reference") (Stimulus :type "AIStimulus Structure"))
  ;[1 1 1] WatchingTimer
  (if (`.bSuccessfullySensed` (break `AIStimulus` Stimulus))
    (bind _returnvalue (`KismetSystemLibrary.K2_SetTimerDelegate` (delegate `WatchingPlayer`) 0.01 true))
    (set `self.Watching` _returnvalue)
    ;[1 1 1] is player close enough to shot
    (if (< (`GameplayStatics.FindNearestActor` (`self.K2_GetActorLocation`) (`|MakeArray` (`self.As BP Third Person Character`) :!type "Actor Object Reference")) 2000.0)
      (bind _returnvalue_2 (`KismetSystemLibrary.K2_SetTimerDelegate` (delegate `Shooting`) 2.0 true))
      (set `self.Shooting timer` _returnvalue_2)
      (else
        (`KismetSystemLibrary.K2_ClearAndInvalidateTimerHandle` (`self.Shooting timer`))))
    (else
      (`KismetSystemLibrary.K2_ClearAndInvalidateTimerHandle` (`self.Watching`))
      (`KismetSystemLibrary.K2_ClearAndInvalidateTimerHandle` (`self.Shooting timer`)))))

(event `Damage`
  (bind _mesh (`self.Mesh`))
  (bind (_returnvalue_roll _returnvalue_pitch _returnvalue_yaw) (`KismetMathLibrary.BreakRotator` (`SceneComponent.K2_GetComponentRotation` _mesh)))
  ;[1 1 1] death
  (`|ExecutionSequence`
    (:`then_0`
      (goto _label :!via `Stop`))
    (:`then_1`
      (bind (_direction _ded) (`Timeline|EnemyDied` :!via `PlayFromStart`)
        (:`Finished`
          (`SceneComponent.K2_SetRelativeRotation` _mesh (`KismetMathLibrary.MakeRotator` _returnvalue_roll (+ _returnvalue_pitch (.y _ded)) (+ _returnvalue_yaw (.z _ded))) false false)
          (`KismetSystemLibrary.Delay` 1.0)
          (`PrimitiveComponent.SetMaterial` (`self.Mesh`) 0 "/Game/Art/Mats/MI_Zombee.MI_Zombee"))))))

(event `WatchingPlayer`
  (bind _as_bp_third_person_character (`self.As BP Third Person Character`))
  ;[1 1 1] watching player
  (`/Engine/EditorBlueprintResources/StandardMacros.IsValid` _as_bp_third_person_character
    (:`Is Valid`
      (`self.K2_SetActorRotation` (`KismetMathLibrary.FindLookAtRotation` (`self.K2_GetActorLocation`) (`self.K2_GetActorLocation` _as_bp_third_person_character))))))

(event `Shooting`
  (bind _as_bp_third_person_character (`self.As BP Third Person Character`))
  ;[1 1 1] shooting
  (`KismetSystemLibrary.K2_ClearAndInvalidateTimerHandle` (`self.Watching`))
  (`GameplayStatics.PlaySoundAtLocation` "/Game/Zombe/Audio/visceralbulletimpacts-6738.visceralbulletimpacts-6738" (`self.K2_GetActorLocation`) (struct) 0.5 1.0 0.0 null null null null)
  (`/Engine/EditorBlueprintResources/StandardMacros.IsValid` _as_bp_third_person_character
    (:`Is Valid`
      (bind _outhit (`KismetSystemLibrary.LineTraceSingle` (`self.K2_GetActorLocation`) (`self.K2_GetActorLocation` _as_bp_third_person_character) "TraceTypeQuery1"))
      (bind (_bblockinghit _binitialoverlap _time _distance _location _impactpoint _normal _impactnormal _physmat _hitactor _hitcomponent _hitbonename _bonename _hititem _elementindex _faceindex _tracestart _traceend) (`GameplayStatics.BreakHitResult` _outhit))
      (`|SpawnActorFromClass` "/Game/Zombe/Fi/BP_Projectile.BP_Projectile_C" (`KismetMathLibrary.MakeTransform` _tracestart (`KismetMathLibrary.FindLookAtRotation` _tracestart _traceend)) "Undefined" "MultiplyWithRoot" null (`self.As BP Third Person Character`) null))))

(fn `UserConstructionScript`)